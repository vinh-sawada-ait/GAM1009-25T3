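; Enemy spawner, named for a wave system, that spawns random enemy types along the line between two arrow components.
; QueueTimer, not called from BeginPlay, starts a self-repeating SpawnEnemy loop with random delays.
; Each spawn receives a drop-on-death pickup from the first passing roll against PickUpChance, with index -1 when none passes.
; All randomness uses one Stream, reset on BeginPlay for repeatable sequences.
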(event Custom|QueueTimer
  (Utilities|Time|SetTimerbyEvent (delegate Custom|SpawnEnemy) (Math|Random|RandomFloatinRangefromStream (Variables|Default|GetStream) 2.0 6.0)))

(event Custom|SpawnEnemy
  (bind _arrowleftside (Variables|Default|GetArrowLeftSide))
  (bind _returnvalue (Transformation|GetWorldLocation _arrowleftside))
  (CallFunction|SelectRandomPickup)
  (Game|SpawnActorfromClass (.OutItem (Utilities|Array|RandomFromStream (Variables|Default|GetEnemyTypes) (Variables|Default|GetStream))) (Math|Transform|MakeTransform (Math|Vector|MakeVector (.x _returnvalue) (Math|Random|RandomFloatinRangefromStream (Variables|Default|GetStream) (.y _returnvalue) (.y (Transformation|GetWorldLocation (Variables|Default|GetArrowRightSide)))) (.z _returnvalue)) (Transformation|GetWorldRotation _arrowleftside) "1.000000,1.000000,1.000000") "Undefined" "MultiplyWithRoot" 0 (Utilities|Array|Get(acopy) (Variables|Default|GetPickUpTypes) (Variables|Default|GetSelectedPickUpIndex)) 0)
  (CallFunction|QueueTimer))

(event Custom|SelectRandomPickup
  (Variables|Default|SetSelectedPickUpIndex -1)
  (bind (_array_element _array_index) (Utilities|Array|ForEachLoopwithBreak (Variables|Default|GetPickUpChance) :!label _label)
    (:LoopBody
      (if (<= (Math|Random|RandomFloatfromStream (Variables|Default|GetStream)) _array_element)
        (Variables|Default|SetSelectedPickUpIndex _array_index)
        (goto _label Break)))))

(event EventBeginPlay
  (Class|KismetMathLibrary|ResetRandomStream (Variables|Default|GetStream)))

(fn ConstructionScript)