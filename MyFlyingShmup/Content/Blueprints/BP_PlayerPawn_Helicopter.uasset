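; Player-controlled helicopter pawn that flies via FloatingPawnMovement and Enhanced Input, with spinning main and stabilizer rotors.
; Move inputs drive forward, sideways and vertical motion, mouse look turns the controller, and primary fire spawns BP_Bullet at a spawn point.
; Each tick smoothly turns the actor toward control yaw and tilts only the Body component in pitch and roll from interpolated movement input.
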(event Custom|SetRotatingParts
  (Components|Movement|SetUpdatedComponent (Variables|Default|GetRotatingMovement) (Variables|Default|GetRotorBase))
  (Components|Movement|SetUpdatedComponent (Variables|Default|GetRotatingMovement1) (Variables|Default|GetStabaliserBase)))

(event Custom|RotatePawnYaw
  (bind _output_get (Variables|Default|SetTargetPawnYaw (.yaw (Pawn|GetControlRotation :!class /Script/Engine.Pawn))))
  (bind _output_get_2 (Variables|Default|SetCurrentPawnYaw (.yaw (Math|Interpolation|RInterpTo (Math|Rotator|MakeRotator 0.0 0.0 (Variables|Default|GetCurrentPawnYaw)) (Math|Rotator|MakeRotator 0.0 0.0 _output_get) (Utilities|Time|GetWorldDeltaSeconds) 2.0))))
  (Transformation|SetActorRotation (Math|Rotator|MakeRotator 0.0 0.0 _output_get_2)))

(event Custom|CalculatePawnPitch
  (bind _output_get (Variables|Default|SetTargetPawnPitch (Input|EnhancedActionValues|GetIA_MoveForwardBackward)))
  (Variables|Default|SetCurrentPawnPitch (Math|Interpolation|FInterpTo (Variables|Default|GetCurrentPawnPitch) _output_get (Utilities|Time|GetWorldDeltaSeconds) 2.0)))

(event Custom|CalculatePawnRoll
  (bind _output_get (Variables|Default|SetTargetPawnRoll (Input|EnhancedActionValues|GetIA_MoveRightLeft)))
  (Variables|Default|SetCurrentPawnRoll (Math|Interpolation|FInterpTo (Variables|Default|GetCurrentPawnRoll) _output_get (Utilities|Time|GetWorldDeltaSeconds) 2.0)))

(event Custom|ApplyPitchRoll
  (Transformation|SetRelativeRotation (Variables|Default|GetBody) (Math|Rotator|MakeRotator (* (Variables|Default|GetCurrentPawnRoll) 3e+01) (* (Variables|Default|GetCurrentPawnPitch) -3e+01) 0.0) false false))

(event Input|EnhancedActionEvents|EnhancedInputActionIA_MoveForwardBackward
  (params (ActionValue :type Float%20%28double-precision%29) (ElapsedSeconds :type Float%20%28double-precision%29) (TriggeredSeconds :type Float%20%28double-precision%29) (InputAction :type Input%20Action%20Object%20Reference :default "/Game/Inputs/IA_MoveForwardBackward.IA_MoveForwardBackward"))
  (Class|PawnMovementComponent|AddInputVector (Variables|Default|GetFloatingPawnMovement) (* ActionValue (Transformation|GetActorForwardVector)) false))

(event Input|EnhancedActionEvents|EnhancedInputActionIA_MoveRightLeft
  (params (ActionValue :type Float%20%28double-precision%29) (ElapsedSeconds :type Float%20%28double-precision%29) (TriggeredSeconds :type Float%20%28double-precision%29) (InputAction :type Input%20Action%20Object%20Reference :default "/Game/Inputs/IA_MoveRightLeft.IA_MoveRightLeft"))
  (Class|PawnMovementComponent|AddInputVector (Variables|Default|GetFloatingPawnMovement) (* ActionValue (Transformation|GetActorRightVector)) false))

(event Input|EnhancedActionEvents|EnhancedInputActionIA_LookWithMouse
  (params (ActionValue :type Vector%202D%20Structure) (ElapsedSeconds :type Float%20%28double-precision%29) (TriggeredSeconds :type Float%20%28double-precision%29) (InputAction :type Input%20Action%20Object%20Reference :default "/Game/Inputs/IA_LookWithMouse.IA_LookWithMouse"))
  (Pawn|Input|AddControllerYawInput (* (.x ActionValue) 1.0))
  (Pawn|Input|AddControllerPitchInput (* (.y ActionValue) -1.0)))

(event Input|EnhancedActionEvents|EnhancedInputActionIA_MoveUpDown
  (params (ActionValue :type Float%20%28double-precision%29) (ElapsedSeconds :type Float%20%28double-precision%29) (TriggeredSeconds :type Float%20%28double-precision%29) (InputAction :type Input%20Action%20Object%20Reference :default "/Game/Inputs/IA_MoveUpDown.IA_MoveUpDown"))
  (Class|PawnMovementComponent|AddInputVector (Variables|Default|GetFloatingPawnMovement) (* ActionValue (Transformation|GetActorUpVector)) false))

(event Input|EnhancedActionEvents|EnhancedInputActionIA_PrimaryFire
  (params (ActionValue :type Boolean) (ElapsedSeconds :type Float%20%28double-precision%29) (TriggeredSeconds :type Float%20%28double-precision%29) (InputAction :type Input%20Action%20Object%20Reference :default "/Game/Inputs/IA_PrimaryFire.IA_PrimaryFire"))
  (bind _primaryfirespawnpoint1 (Variables|Default|GetPrimaryFireSpawnPoint1))
  (bind _returnvalue (Transformation|GetWorldTransform _primaryfirespawnpoint1))
  (Game|SpawnActorfromClass "/Game/Blueprints/BP_Bullet.BP_Bullet_C" (Math|Transform|MakeTransform (.location _returnvalue) (.rotation _returnvalue) "1.000000,1.000000,1.000000") "Undefined" "MultiplyWithRoot" 0 0))

(event EventBeginPlay
  (CallFunction|SetRotatingParts))

(event EventPossessed
  (params (NewController :type Controller%20Object%20Reference))
  (bind _asplayer_controller (Utilities|Casting|CastToPlayerController NewController))
  (bind _output_get (Variables|Default|SetPlayerController _asplayer_controller))
  (Input|AddMappingContext (PlayerController|LocalPlayerSubsystems|GetEnhancedInputLocalPlayerSubsystem _output_get) "/Game/Inputs/IMC_PlayerInputs.IMC_PlayerInputs" 0 "(bIgnoreAllPressedKeysUntilRelease=True,bForceImmediately=False,bNotifyUserSettings=False)"))

(event EventTick
  (params (DeltaSeconds :type Float%20%28single-precision%29))
  (CallFunction|RotatePawnYaw)
  (CallFunction|CalculatePawnPitch)
  (CallFunction|CalculatePawnRoll)
  (CallFunction|ApplyPitchRoll))

(fn ConstructionScript)