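; Player-controlled dual-rotor helicopter pawn that flies with Enhanced Input and a FloatingPawnMovement component.
; Movement actions add input along the actor's forward, right and vertical axes, while mouse look drives the control rotation.
; Each tick the pawn's yaw smoothly follows the control yaw, and the body mesh eases into pitch and roll tilt from movement input.
; Two RotatingMovement components, assigned on BeginPlay, spin the front and rear rotors.
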(event Custom|SetRotatingComponents
  (Components|Movement|SetUpdatedComponent (Variables|Default|GetRotatingMovement1) (Variables|Default|GetFrontRotorBase))
  (Components|Movement|SetUpdatedComponent (Variables|Default|GetRotatingMovement) (Variables|Default|GetRearRotorBase)))

(event Custom|RotatePawnYaw
  (bind _output_get (Variables|Default|SetTargetPawnYaw (.yaw (Pawn|GetControlRotation :!class /Script/Engine.Pawn))))
  (bind _output_get_2 (Variables|Default|SetCurrentPawnYaw (.yaw (Math|Interpolation|RInterpTo (Math|Rotator|MakeRotator 0.0 0.0 (Variables|Default|GetCurrentPawnYaw)) (Math|Rotator|MakeRotator 0.0 0.0 _output_get) (Utilities|Time|GetWorldDeltaSeconds) 2.0))))
  (Transformation|SetActorRotation (Math|Rotator|MakeRotator 0.0 0.0 _output_get_2)))

(event Custom|CalcBodyPitch
  (bind _output_get (Variables|Default|SetTargetBodyPitch (Input|EnhancedActionValues|GetIA_MoveForwardBackward)))
  (Variables|Default|SetCurrentBodyPitch (Math|Interpolation|FInterpTo (Variables|Default|GetCurrentBodyPitch) _output_get (Utilities|Time|GetWorldDeltaSeconds) 1.0)))

(event Custom|CalcBodyRoll
  (bind _output_get (Variables|Default|SetTargetBodyRoll (Input|EnhancedActionValues|GetIA_MoveRightLeft)))
  (Variables|Default|SetCurrentBodyRoll (Math|Interpolation|FInterpTo (Variables|Default|GetCurrentBodyRoll) _output_get (Utilities|Time|GetWorldDeltaSeconds) 1.0)))

(event Custom|RotateBodyPitchAndRoll
  (Transformation|SetRelativeRotation (Variables|Default|GetBody) (Math|Rotator|MakeRotator (* (Variables|Default|GetCurrentBodyRoll) 3e+01) (* (Variables|Default|GetCurrentBodyPitch) -15.0) 0.0) false false))

(event Input|EnhancedActionEvents|EnhancedInputActionIA_MoveForwardBackward
  (params (ActionValue :type Float%20%28double-precision%29) (ElapsedSeconds :type Float%20%28double-precision%29) (TriggeredSeconds :type Float%20%28double-precision%29) (InputAction :type Input%20Action%20Object%20Reference :default "/Game/Inputs/IA_MoveForwardBackward.IA_MoveForwardBackward"))
  (Class|PawnMovementComponent|AddInputVector (Variables|Default|GetFloatingPawnMovement) (* ActionValue (Transformation|GetActorForwardVector)) false))

(event Input|EnhancedActionEvents|EnhancedInputActionIA_MoveRightLeft
  (params (ActionValue :type Float%20%28double-precision%29) (ElapsedSeconds :type Float%20%28double-precision%29) (TriggeredSeconds :type Float%20%28double-precision%29) (InputAction :type Input%20Action%20Object%20Reference :default "/Game/Inputs/IA_MoveRightLeft.IA_MoveRightLeft"))
  (Class|PawnMovementComponent|AddInputVector (Variables|Default|GetFloatingPawnMovement) (* ActionValue (Transformation|GetActorRightVector)) false))

(event Input|EnhancedActionEvents|EnhancedInputActionIA_MoveUpDown
  (params (ActionValue :type Float%20%28double-precision%29) (ElapsedSeconds :type Float%20%28double-precision%29) (TriggeredSeconds :type Float%20%28double-precision%29) (InputAction :type Input%20Action%20Object%20Reference :default "/Game/Inputs/IA_MoveUpDown.IA_MoveUpDown"))
  (Class|PawnMovementComponent|AddInputVector (Variables|Default|GetFloatingPawnMovement) (Math|Vector|MakeVector 0.0 0.0 ActionValue) false))

(event Input|EnhancedActionEvents|EnhancedInputActionIA_LookWithMouse
  (params (ActionValue :type Vector%202D%20Structure) (ElapsedSeconds :type Float%20%28double-precision%29) (TriggeredSeconds :type Float%20%28double-precision%29) (InputAction :type Input%20Action%20Object%20Reference :default "/Game/Inputs/IA_LookWithMouse.IA_LookWithMouse"))
  (Pawn|Input|AddControllerYawInput (.x ActionValue))
  (Pawn|Input|AddControllerPitchInput (* (.y ActionValue) -1.0)))

(event EventBeginPlay
  (CallFunction|SetRotatingComponents))

(event EventPossessed
  (params (NewController :type Controller%20Object%20Reference))
  (bind _asplayer_controller (Utilities|Casting|CastToPlayerController NewController))
  (Input|AddMappingContext (PlayerController|LocalPlayerSubsystems|GetEnhancedInputLocalPlayerSubsystem _asplayer_controller) "/Game/Inputs/IMC_PlayerInputs.IMC_PlayerInputs" 0 "(bIgnoreAllPressedKeysUntilRelease=True,bForceImmediately=False,bNotifyUserSettings=False)"))

(event EventTick
  (params (DeltaSeconds :type Float%20%28single-precision%29))
  (CallFunction|RotatePawnYaw)
  (CallFunction|CalcBodyPitch)
  (CallFunction|CalcBodyRoll)
  (CallFunction|RotateBodyPitchandRoll))

(fn ConstructionScript)