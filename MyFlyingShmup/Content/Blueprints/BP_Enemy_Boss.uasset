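; Boss enemy Blueprint that scripts the boss's movement from BeginPlay in two timeline-driven phases.
; The first timeline runs at half speed, moving the actor along its Spline at constant velocity relative to its starting transform.
; When it finishes, the current transform becomes the new origin and the LeftToRight timeline offsets the boss along that transform's local Y axis.
; Both phases use swept transform updates.
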(event EventBeginPlay
  (|CallParentFunction)
  (Components|Timeline|SetPlayRate (Variables|Default|GetTimeline) 0.5)
  (Variables|Default|SetInitialTransform (Transformation|GetActorTransform))
  (bind _progress (Timeline|Timeline PlayFromStart)
    (:Update
      (bind _spline (Variables|Default|GetSpline)
        (:then
          (Transformation|SetActorTransform (Math|Transform|MakeRelativeTransform (Variables|Default|GetInitialTransform) (Math|Transform|MakeTransform (Spline|GetLocationatTime _spline _progress "Local" true))) true))
        (:else)))
    (:Finished
      (Variables|Default|SetInitialTransform (Transformation|GetActorTransform))
      (bind _value (Timeline|LeftToRight PlayFromStart)
        (:Update
          (Transformation|SetActorTransform (Math|Transform|MakeRelativeTransform (Math|Transform|MakeTransform (Math|Vector|MakeVector 0.0 (* _value 8e+02) 0.0) "0, 0, 0" "1.000000,1.000000,1.000000") (Variables|Default|GetInitialTransform)) true))))))

(event Collision|EventActorBeginOverlap
  (params (OtherActor :type Actor%20Object%20Reference))
  (|CallParentFunction OtherActor) ; This node is disabled and will not be called.\nDrag off pins to build functionality.
)

(event EventTick
  (params (DeltaSeconds :type Float%20%28single-precision%29)))

(fn ConstructionScript
  (|CallParentFunction))