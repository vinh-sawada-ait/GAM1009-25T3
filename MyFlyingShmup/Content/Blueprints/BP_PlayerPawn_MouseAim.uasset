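; Player pawn for a flying shoot-'em-up that moves via Enhanced Input and yaws toward the cursor's trace point each tick.
; Primary fire spawns bullets in three debug-switchable modes: single, alternating muzzles or angled spray.
; Damage drives camera shake, overlay flash and HUD health, while overlaps damage the other actor by this pawn's health.
; Death spawns and possesses a replacement at PlayerStart, with sphere collision briefly disabled on BeginPlay.
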(event Custom|ApplyCameraShake
  (Camera|PlayWorldCameraShake "/Game/Blueprints/BP_CameraShake.BP_CameraShake_C" "0, 0, 0" 0.0 1e+04))

(event Custom|CheckHealth
  (CallFunction|UpdateHUD)
  (if (== (Variables|Default|GetHealth) 0.0)
    (CallFunction|OnDeath)))

(event Custom|OnDeath
  (bind _returnvalue (Actor|GetActorOfClass "/Script/Engine.PlayerStart"))
  (Utilities|IsValid _returnvalue
    (:Is%20Valid
      (bind _returnvalue_2 (Game|SpawnActorfromClass "BP_PlayerPawn_MouseAim_C" (Transformation|GetActorTransform _returnvalue) "AlwaysSpawn" "MultiplyWithRoot" 0 0))
      (bind _asplayer_controller (Utilities|Casting|CastToPlayerController (Pawn|GetController)))
      (Pawn|Possess _asplayer_controller _returnvalue_2)
      (Actor|DestroyActor)
      (Niagara|SpawnSystematLocation "/Game/Particles/FX_EnemyExplosion_System.FX_EnemyExplosion_System" (Transformation|GetActorLocation)))))

(event Custom|FlashRedOverlayMaterial
  (Rendering|Material|SetOverlayMaterial (Variables|Default|GetMesh) "/Game/Materials/M_OverlayWhenHit.M_OverlayWhenHit" :!class /Script/Engine.MeshComponent)
  (Utilities|FlowControl|Delay 0.2)
  (Rendering|Material|SetOverlayMaterial (Variables|Default|GetMesh) 0 :!class /Script/Engine.MeshComponent))

(event Custom|UpdateHUD
  (bind _ashud_my_flying_shmup (Utilities|Casting|CastToHUD_MyFlyingShmup (HUD|GetHUD (Variables|Default|GetAsPlayer%20Controller))))
  (Utilities|IsValid (Variables|/Game/Core/HUD_MyFlyingShmup.HUD_MyFlyingShmup_C|GetPlayerWidget _ashud_my_flying_shmup)
    (:Is%20Valid
      (Default|SetHealthPercent (Variables|/Game/Core/HUD_MyFlyingShmup.HUD_MyFlyingShmup_C|GetPlayerWidget _ashud_my_flying_shmup) (Math|Float|SafeDivide (Variables|Default|GetHealth) (Variables|Default|GetMaxHealth))))))

(event Input|EnhancedActionEvents|EnhancedInputActionIA_MoveForwardBackward
  (params (ActionValue :type Float%20%28double-precision%29) (ElapsedSeconds :type Float%20%28double-precision%29) (TriggeredSeconds :type Float%20%28double-precision%29) (InputAction :type Input%20Action%20Object%20Reference :default "/Game/Inputs/IA_MoveForwardBackward.IA_MoveForwardBackward"))
  (Class|PawnMovementComponent|AddInputVector (Variables|Default|GetFloatingPawnMovement) (Math|Vector|MakeVector ActionValue 0.0 0.0) false))

(event Input|EnhancedActionEvents|EnhancedInputActionIA_MoveRightLeft
  (params (ActionValue :type Float%20%28double-precision%29) (ElapsedSeconds :type Float%20%28double-precision%29) (TriggeredSeconds :type Float%20%28double-precision%29) (InputAction :type Input%20Action%20Object%20Reference :default "/Game/Inputs/IA_MoveRightLeft.IA_MoveRightLeft"))
  (Class|PawnMovementComponent|AddInputVector (Variables|Default|GetFloatingPawnMovement) (Math|Vector|MakeVector 0.0 ActionValue 0.0) false))

(event Input|EnhancedActionEvents|EnhancedInputActionIA_PrimaryFire
  (params (ActionValue :type Boolean) (ElapsedSeconds :type Float%20%28double-precision%29) (TriggeredSeconds :type Float%20%28double-precision%29) (InputAction :type Input%20Action%20Object%20Reference :default "/Game/Inputs/IA_PrimaryFire.IA_PrimaryFire"))
  (bind _arrow (Variables|Default|GetArrow))
  (bind _arrow_2 (Variables|Default|GetArrow))
  (bind _returnvalue (Math|Vector|GetForwardVector _arrow_2))
  (bind _returnvalue_2 (Transformation|GetWorldTransform _arrow))
  (bind _returnvalue_3 (Math|Rotator|MakeRotfromX _returnvalue))
  (Utilities|FlowControl|Delay 0.2)
  (switch int (Variables|Default|GetShootingModeIndex)
    (:0
      ;[0.15 0.15 0.15 0.5] Shooting Mode 1
      (Game|SpawnActorfromClass "/Game/Blueprints/BP_Bullet_2D_Player.BP_Bullet_2D_Player_C" (Math|Transform|MakeTransform (.location _returnvalue_2) (.rotation _returnvalue_2) "1.000000,1.000000,1.000000") "Undefined" "MultiplyWithRoot" 0 0))
    (:1
      ;[0.15 0.15 0.15 0.5] Shooting Mode 2
      (bind _isa (Utilities|FlowControl|FlipFlop)
        (:A
          _)
        (:B
          _))
      (Game|SpawnActorfromClass "/Game/Blueprints/BP_Bullet_2D_Player.BP_Bullet_2D_Player_C" (Math|Transform|MakeTransform (.location (Transformation|GetWorldTransform (select _isa (Variables|Default|GetPrimaryFireSpawnPoint2) (Variables|Default|GetPrimaryFireSpawnPoint1)))) (.rotation (Transformation|GetWorldTransform (select _isa (Variables|Default|GetPrimaryFireSpawnPoint2) (Variables|Default|GetPrimaryFireSpawnPoint1)))) "1.000000,1.000000,1.000000") "Undefined" "MultiplyWithRoot" 0 0))
    (:2
      ;[0.15 0.15 0.15 0.5] Shooting Mode 3
      (for _index (range 1 (Variables|Default|GetNumberOfBulletsToSpray))
        (Game|SpawnActorfromClass "/Game/Blueprints/BP_Bullet_2D_Player.BP_Bullet_2D_Player_C" (Math|Transform|MakeTransform (Transformation|GetWorldLocation _arrow_2) (Math|Rotator|MakeRotator (.roll _returnvalue_3) (.pitch _returnvalue_3) (+ (.yaw _returnvalue_3) (Utilities|Operators|Subtract (* _index (Variables|Default|GetAngleOfSprayedBullets)) (* (Math|Float|Round (* (Variables|Default|GetNumberOfBulletsToSpray) 0.5)) (Variables|Default|GetAngleOfSprayedBullets))))) "1.000000,1.000000,1.000000") "Undefined" "MultiplyWithRoot" 0 0)))))

(event Collision|EventActorBeginOverlap
  (params (OtherActor :type Actor%20Object%20Reference))
  (Game|Damage|ApplyDamage OtherActor (Variables|Default|GetHealth) 0 0))

(event Game|Damage|EventAnyDamage
  (params (Damage :type Float%20%28single-precision%29) (DamageType :type Damage%20Type%20Object%20Reference) (InstigatedBy :type Controller%20Object%20Reference) (DamageCauser :type Actor%20Object%20Reference))
  (bind _output_get (Variables|Default|SetHealth (Math|Float|Clamp(Float) (- (Variables|Default|GetHealth) Damage) 0.0 (Variables|Default|GetMaxHealth))))
  (CallFunction|ApplyCameraShake)
  (CallFunction|FlashRedOverlayMaterial)
  (Development|PrintString (Utilities|String|ToString(Float) _output_get))
  (CallFunction|CheckHealth))

(event EventBeginPlay
  (Collision|SetCollisionEnabled (Variables|Default|GetSphere) "NoCollision")
  (Utilities|FlowControl|Delay 2.0)
  (Collision|SetCollisionEnabled (Variables|Default|GetSphere) "QueryAndPhysics")
  (Variables|/Script/Engine.PlayerController|SetbShowMouseCursor (Variables|Default|GetAsPlayer%20Controller) true)
  (Variables|/Script/Engine.PlayerController|SetCurrentMouseCursor (Variables|Default|GetAsPlayer%20Controller) "Crosshairs"))

(event EventPossessed
  (params (NewController :type Controller%20Object%20Reference))
  (bind _asplayer_controller (Utilities|Casting|CastToPlayerController NewController))
  (bind _output_get (Variables|Default|SetAsPlayer%20Controller _asplayer_controller))
  (Input|AddMappingContext (PlayerController|LocalPlayerSubsystems|GetEnhancedInputLocalPlayerSubsystem _output_get) "/Game/Inputs/IMC_PlayerInputs.IMC_PlayerInputs" 0 "(bIgnoreAllPressedKeysUntilRelease=True,bForceImmediately=False,bNotifyUserSettings=False)")
  (CallFunction|CheckHealth))

(event EventTick
  (params (DeltaSeconds :type Float%20%28single-precision%29))
  (Transformation|SetWorldLocation (Variables|Default|GetMouseTarget) (.Location (Collision|BreakHitResult (.HitResult (Game|Player|GetHitResultUnderCursorbyChannel (Variables|Default|GetAsPlayer%20Controller) "TraceTypeQuery1" false)))) false false)
  (Transformation|SetActorRotation (Math|Rotator|MakeRotator 0.0 0.0 (.yaw (Math|Rotator|FindLookatRotation (Transformation|GetActorLocation) (Transformation|GetWorldLocation (Variables|Default|GetMouseTarget)))))))

(event Input|KeyboardEvents|DebugKeyM
  (params (Key :type Key%20Structure :default "None") (ActionValue :type Input%20Action%20Value%20Structure))
  (:Pressed
    (Variables|Default|SetShootingModeIndex (Math|Integer|Clamp(Integer) (+ (Variables|Default|GetShootingModeIndex) 1) -1 2))))

(event Input|KeyboardEvents|DebugKeyN
  (params (Key :type Key%20Structure :default "None") (ActionValue :type Input%20Action%20Value%20Structure))
  (:Pressed
    (Variables|Default|SetShootingModeIndex (Math|Integer|Clamp(Integer) (- (Variables|Default|GetShootingModeIndex) 1) -1 2))))

(fn ConstructionScript)